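; AI controller for the Freddy Fazbear enemy that runs its behavior tree and turns AI perception into blackboard targets.
; Sight sets TargetActor, or on losing sight clears it and stores the player's current location as InvestigationLocation.
; Hearing stores the noise location as InvestigationLocation.
; When perception updates while the player's BP_Zion has MaskON, both keys are cleared instead, so the mask hides the player.
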(event `self.ReceiveBeginPlay`
  (`self.RunBehaviorTree` "/Game/BP/Enemy/BT_FreddyFazbear.BT_FreddyFazbear"))

(event `self.AIPerception.OnTargetPerceptionUpdated`
  (params (Actor :type "Actor Object Reference") (Stimulus :type "AIStimulus Structure"))
  ;[1 1 1] Detect Player
  (if (`/Game/BP/FirstPerson/Blueprints/BP_Zion.MaskON` (cast `/Game/BP/FirstPerson/Blueprints/BP_Zion` (`GameplayStatics.GetPlayerPawn` 0) :!pure true))
    (`self.PutMaskOn`)
    (else
      (`self.Sight_Detection` Actor Stimulus)
      (`self.Hearing_Detection` Actor Stimulus))))

(fn `Hearing_Detection`
  (params (F_Actor :type "Actor Object Reference") (F_Stimulus :type "AIStimulus Structure"))
  (bind _returnvalue (`AIPerceptionSystem.GetSenseClassForStimulus` F_Stimulus))
  (if (== _returnvalue "/Script/AIModule.AISense_Hearing")
    (`BlackboardComponent.SetValueAsVector` (`AIBlueprintHelperLibrary.GetBlackboard` null) "InvestigationLocation" (`.StimulusLocation` (break `AIStimulus` F_Stimulus)))))

(fn `PutMaskOn`
  (`BlackboardComponent.ClearValue` (`AIBlueprintHelperLibrary.GetBlackboard` null) "InvestigationLocation")
  (`BlackboardComponent.SetValueAsObject` (`AIBlueprintHelperLibrary.GetBlackboard` null) "TargetActor" null))

(fn `Sight_Detection`
  (params (F_Actor :type "Actor Object Reference") (F_Stimulus :type "AIStimulus Structure (by ref)"))
  (bind _returnvalue (`AIPerceptionSystem.GetSenseClassForStimulus` F_Stimulus))
  (if (== _returnvalue "/Script/AIModule.AISense_Sight")
    (if (`.bSuccessfullySensed` (break `AIStimulus` F_Stimulus))
      (`BlackboardComponent.SetValueAsObject` (`AIBlueprintHelperLibrary.GetBlackboard` null) "TargetActor" F_Actor)
      (else
        (`BlackboardComponent.SetValueAsObject` (`AIBlueprintHelperLibrary.GetBlackboard` null) "TargetActor" null)
        (`BlackboardComponent.SetValueAsVector` (`AIBlueprintHelperLibrary.GetBlackboard` null) "InvestigationLocation" (`self.K2_GetActorLocation` (`GameplayStatics.GetPlayerPawn` 0)))))))

(fn `UserConstructionScript`)