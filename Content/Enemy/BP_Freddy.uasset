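; Freddy Fazbear enemy that laughs at random intervals, shakes the camera with its steps and hosts an interactive minigame.
; Interact locks the BP_Zion player, blends the view to Freddy and shows the Minig widget with mouse input; quitfreddy reverses this.
; Stun sets a Blackboard key for the AI, plus a big or small flag with matching screams.
; The construction script snaps eye spheres and spotlights to mesh sockets.
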(event `openminigame`
  (`PrimitiveComponent.SetCollisionResponseToChannel` (`self.Mesh`) "ECC_GameTraceChannel2" "ECR_Block"))

(event `endminigame`
  (`PrimitiveComponent.SetCollisionResponseToChannel` (`self.Mesh`) "ECC_GameTraceChannel2" "ECR_Ignore"))

(event `self.ReceiveBeginPlay`
  (`GameplayStatics.PlaySoundAtLocation` "/Game/BP/Sfx/FreddyLaugh.FreddyLaugh" (`self.K2_GetActorLocation`) (struct) 1.0 1.0 0.0 "/Game/BP/Sfx/atenuationlaugh.atenuationlaugh" null null null :!label _label)
  (`KismetSystemLibrary.Delay` (`KismetMathLibrary.RandomFloatInRange` 10.0 30.0))
  (goto _label))

(event `/Game/BP/InteractionSystem/IInteractable.interact`
  (bind _returnvalue (`GameplayStatics.GetPlayerController` 0))
  (bind _minig (`self.minig`))
  (bind _mesh (`self.Mesh`))
  (bind (_relativelocation_x _relativelocation_y) (`KismetMathLibrary.BreakVector` (`SceneComponent.RelativeLocation` _mesh)))
  (if (not (`self.Interracted`))
    (set `self.Interracted` true)
    (set `/Game/BP/FirstPerson/Blueprints/BP_Zion.interracted` true (cast `/Game/BP/FirstPerson/Blueprints/BP_Zion` (`GameplayStatics.GetPlayerPawn` 0) :!pure true))
    (`SkeletalMeshComponent.SetAnimInstanceClass` (`self.Mesh`) null)
    (`SceneComponent.K2_SetRelativeLocation` _mesh (`KismetMathLibrary.MakeVector` _relativelocation_x _relativelocation_y) false false)
    (`/Game/BP/FirstPerson/Blueprints/BP_Zion.remove mask` (cast `/Game/BP/FirstPerson/Blueprints/BP_Zion` (`GameplayStatics.GetPlayerPawn` 0) :!pure true))
    (`GameplayStatics.PlaySoundAtLocation` "/Game/BP/Sfx/openholo.openholo" (`self.K2_GetActorLocation`) (struct) 1.0 1.0 0.0 null null null null)
    (`SceneComponent.SetVisibility` _minig true false)
    (`PlayerController.SetViewTargetWithBlend` _returnvalue self 0.25 "VTBlend_Linear" 0.0 false)
    (`PrimitiveComponent.SetCollisionResponseToChannel` _minig "ECC_Visibility" "ECR_Block")
    (`WidgetBlueprintLibrary.SetInputMode_GameAndUIEx` _returnvalue (`WidgetComponent.GetWidget` _minig) "DoNotLock" false)
    (set `PlayerController.bShowMouseCursor` true _returnvalue)
    (`KismetSystemLibrary.Delay` 0.2)
    (set `self.start game` true)))

(event `quit freddy`
  (bind _returnvalue (`GameplayStatics.GetPlayerController` 0))
  (bind _mesh (`self.Mesh`))
  (bind _minig (`self.minig`))
  (bind _asbp_zion (cast `/Game/BP/FirstPerson/Blueprints/BP_Zion` (`GameplayStatics.GetPlayerPawn` 0) :!pure true))
  (bind (_relativelocation_x _relativelocation_y) (`KismetMathLibrary.BreakVector` (`SceneComponent.RelativeLocation` _mesh)))
  (set `self.Interracted` false)
  (set `self.start game` false)
  (`SkeletalMeshComponent.SetAnimInstanceClass` (`self.Mesh`) "/Game/Enemy/Animations/ABP_FreddyFazbear.ABP_FreddyFazbear_C")
  (`SceneComponent.K2_SetRelativeLocation` _mesh (`KismetMathLibrary.MakeVector` _relativelocation_x _relativelocation_y -85.0) false false)
  (set `/Game/BP/FirstPerson/Blueprints/BP_Zion.interracted` false (cast `/Game/BP/FirstPerson/Blueprints/BP_Zion` (`GameplayStatics.GetPlayerPawn` 0) :!pure true))
  (`GameplayStatics.PlaySoundAtLocation` "/Game/BP/Sfx/closehohlo.closehohlo" (`self.K2_GetActorLocation`) (struct) 1.0 1.0 0.0 null null null null)
  (`PlayerController.SetViewTargetWithBlend` _returnvalue _asbp_zion 0.25 "VTBlend_Linear" 0.0 false)
  (`WidgetBlueprintLibrary.SetInputMode_GameOnly` _returnvalue)
  (set `PlayerController.bShowMouseCursor` false _returnvalue)
  (`SceneComponent.SetVisibility` _minig false false)
  (`PrimitiveComponent.SetCollisionResponseToChannel` _minig "ECC_Visibility" "ECR_Ignore")
  (`self.endminigame`)
  (`/Game/BP/FirstPerson/Blueprints/BP_Zion.Endfreddy` _asbp_zion))

(event `Stun`
  (params (`Big?` :type Boolean))
  (`BlackboardComponent.SetValueAsBool` (`AIBlueprintHelperLibrary.GetBlackboard` null) "Stun?" true)
  (if `Big?`
    (set `self.BigStun` true)
    (`GameplayStatics.PlaySoundAtLocation` "/Game/BP/Sfx/freddy_scream.freddy_scream" (`self.K2_GetActorLocation`) (struct) 1.0 1.0 0.0 "/Game/BP/Sfx/Bigatenuation1.Bigatenuation1" null null null)
    (else
      (set `self.Stun?` true)
      (`GameplayStatics.PlaySoundAtLocation` "/Game/BP/Sfx/freddy_scream2.freddy_scream2" (`self.K2_GetActorLocation`) (struct) 1.0 1.0 0.0 "/Game/BP/Sfx/Bigatenuation1.Bigatenuation1" null null null)
      (`GameplayStatics.PlaySoundAtLocation` "/Game/BP/Sfx/screamlittle.screamlittle" (`self.K2_GetActorLocation`) (struct) 1.0 1.0 0.0 "/Game/BP/Sfx/Bigatenuation1.Bigatenuation1" null null null))))

(event `playstepcamerashake`
  (`GameplayStatics.PlayWorldCameraShake` "/Game/BP/Shakes/LoudFreddyStep.LoudFreddyStep_C" (`self.K2_GetActorLocation`) 500.0 3200.0))

(fn `getInfos`
  (params (ObjectName :type Name))
  (returns (ObjectInfos :type "/Game/BP/InteractionSystem/Datas/F_InteractableProps Structure"))
  (return))

(fn `UserConstructionScript`
  (`SceneComponent.K2_AttachToComponent` (`self.Sphere1`) (`self.Mesh`) "L_Eye" "SnapToTarget" "SnapToTarget" "SnapToTarget" true)
  (`SceneComponent.K2_AttachToComponent` (`self.Sphere`) (`self.Mesh`) "R_Eye" "SnapToTarget" "SnapToTarget" "SnapToTarget" true)
  (`SceneComponent.K2_AttachToComponent` (`self.SpotLight1`) (`self.Mesh`) "L_EyeS" "SnapToTarget" "SnapToTarget" "SnapToTarget" true)
  (`SceneComponent.K2_AttachToComponent` (`self.SpotLight`) (`self.Mesh`) "R_EyeS" "SnapToTarget" "SnapToTarget" "SnapToTarget" true))